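; Question countdown Blueprint that shows the time running down on a quiz question as a shrinking cylinder.
; On BeginPlay it saves the cylinder's default scale and binds to the GameState's countdown-change and new-question events.
; Each countdown change lowers the Z scale by a fixed step, while a new question restores the default scale and resets the tracked value to one.
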(event Custom|newQuestion_Event_0
  (params (question :type String) (index :type Integer))
  (Transformation|SetRelativeScale3D (Variables|Default|GetCylinder) (Variables|Default|GetDefaultScale))
  (Variables|Default|SetScale 1.0))

(event Custom|questionCountdownChange_Event_0
  (bind _defaultscale (Variables|Default|GetDefaultScale))
  (bind (_x _y) (Math|Vector|BreakVector _defaultscale))
  (bind _output_get (Variables|Default|SetScale (- (Variables|Default|GetScale) 0.05)))
  (Transformation|SetRelativeScale3D (Variables|Default|GetCylinder) (Math|Vector|MakeVector _x _y _output_get)))

(event EventBeginPlay
  (EventDispatchers|AssignQuestionCountdownChange (Variables|Default|GetGame%20State) (delegate Custom|questionCountdownChange_Event_0))
  (Variables|Default|SetDefaultScale (Variables|/Script/Engine.SceneComponent|GetRelativeScale3D (Variables|Default|GetCylinder)))
  (EventDispatchers|AssignNewQuestion (Variables|Default|GetGame%20State) (delegate Custom|newQuestion_Event_0)))

(fn ConstructionScript)