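; Quiz game state that steps through a question-and-answer map, checks answers, times each question and keeps the score.
; On BeginPlay, chained collapsed graphs bind to event dispatchers, which drive the flow and broadcast results.
; Each answer stops the looping countdown timer and requests the next question after a delay, ending the game when none remain.
; Score resets high, then drops with each countdown tick and more sharply on wrong answers.
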(event EventBeginPlay
  (|NextQuestion
    (:init
      (|NewAnswer
        (:init
          (|Reset-gotostart)
          (|QuestionTimeout :!label _label)
          (|Calculatescore))
        (:newAnswer
          (Utilities|FlowControl|Sequence
            (:then_0
              (Utilities|FlowControl|Delay 2.0)
              (Default|CallNewQuestionRequest))
            (:then_1
              (goto _label execute2))))))))

(fn ConstructionScript)

(event Custom|newAnswer_Event
  (params (alt :type Integer))
  (Utilities|FlowControl|Sequence
    (:then_0
      (if (== (Utilities|Array|Get(acopy) (stale _values) (Variables|Default|GetcurrentQuestionIndex)) alt)
        (Default|CallOnCorrectAnswer)
        (else
          (Default|CallOnWrongAnswer))))
    (:then_1
      (|Outputs) ; enters at newAnswer
    )))

(event Custom|newQuestionRequest_event_345
  (Variables|Default|SetcurrentQuestionIndex (+ (Variables|Default|GetcurrentQuestionIndex) 1))
  (if (>= (Utilities|Map|Length (Variables|Default|Getquestions)) (+ (Variables|Default|GetcurrentQuestionIndex) 1))
    (Default|CallNewQuestion (Utilities|Array|Get(acopy) (stale _keys) (Variables|Default|GetcurrentQuestionIndex)) (Variables|Default|GetcurrentQuestionIndex))
    (|Outputs) ; enters at nextQuestion
    (else
      (Default|CallGameEnded))))

(event Custom|reset_Event
  (Variables|Default|SetcurrentQuestionIndex -1))

(event Custom|reset_Event_2
  (Utilities|Time|ClearandInvalidateTimerbyHandle (stale Custom|newQuestion_Event _returnvalue)))

(event Custom|questionCountdown_Event_1234
  (Utilities|FlowControl|Sequence
    (:then_0
      (bind _output_get (Variables|Default|SetremainingQuestionTime (- (Variables|Default|GetremainingQuestionTime) 0.01)))
      (if (< _output_get 0.0)
        (Utilities|FlowControl|Sequence
          (:then_0
            (Utilities|Time|ClearandInvalidateTimerbyHandle (stale Custom|newQuestion_Event _returnvalue)))
          (:then_1
            (Default|CallQuestionTimeout)))))
    (:then_1
      (Default|CallQuestionCountdownChange))))

(event Custom|nextQuestion_Event_2
  (Variables|Default|SetremainingQuestionTime 1.0))

(event Custom|newQuestion_Event
  (params (question :type String) (index :type Integer))
  (bind _returnvalue (Utilities|Time|SetTimerbyEvent (delegate Custom|questionCountdown_Event_1234) 0.1 true)))

(event Custom|reset_Event_123u
  (bind _output_get (Variables|Default|Setscore 10000))
  (Default|CallScoreUpdate _output_get))

(event Custom|questionCountdownChange_Event
  (bind _output_get (Variables|Default|Setscore (- (Variables|Default|Getscore) 1)))
  (Default|CallScoreUpdate _output_get))

(event Custom|onWrongAnswer_Event
  (bind _output_get (Variables|Default|Setscore (- (Variables|Default|Getscore) 1000)))
  (Default|CallScoreUpdate _output_get))